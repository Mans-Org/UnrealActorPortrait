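; BP_ActorPortrait_SkySphere is the sky sphere backdrop for actor portrait scenes, showing a tinted, rotatable environment cubemap.
; The construction script creates a dynamic instance of the portrait sky material and applies a default gray-light cubemap.
; Portrait scene updates pass environment settings to RefreshSky, which synchronously loads the cubemap and sets the material's texture, tint and rotation.
; The sphere is hidden when no valid cubemap loads.
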(event Custom|Refresh%20Sky
  (params (Asset :type Object%20Soft%20Object%20Reference) (Tint :type Linear%20Color%20Structure) (CubemapRotation :type Float%20%28single-precision%29))
  (bind _returnvalue (Utilities|LoadAssetBlocking Asset))
  (Rendering|SetVisibility (Variables|Default|GetSkySphereMesh) (Utilities|IsValid _returnvalue) false)
  (if (Utilities|IsValid _returnvalue)
    (Rendering|Material|SetVectorParameterValue (Variables|Default|GetSky%20material) "Tint" Tint :!class /Script/Engine.MaterialInstanceDynamic)
    (Rendering|Material|SetScalarParameterValue (Variables|Default|GetSky%20material) "CubemapRotation" CubemapRotation :!class /Script/Engine.MaterialInstanceDynamic)
    (Rendering|Material|SetTextureParameterValue (Variables|Default|GetSky%20material) "Skybox" (.AsTexture (Utilities|Casting|CastToTexture _returnvalue)))))

(event EventOnUpdatePortraitScene
  (params (UserData :type Object%20Object%20Reference))
  (bind _asportrait_environment_settings (Utilities|Casting|CastToPortraitEnvironmentSettings UserData))
  (CallFunction|RefreshSky (Variables|/Script/ActorPortrait.PortraitEnvironmentSettings|GetEnvironmentCubeMap _asportrait_environment_settings) (Variables|/Script/ActorPortrait.PortraitEnvironmentSettings|GetEnvironmentColor _asportrait_environment_settings) (Variables|/Script/ActorPortrait.PortraitEnvironmentSettings|GetEnvironmentRotation _asportrait_environment_settings)))

(fn ConstructionScript
  (bind _returnvalue (Rendering|Material|CreateDynamicMaterialInstance (Variables|Default|GetSkySphereMesh) 0 "/ActorPortrait/SkySphere/M_ActorPortrait_Sky.M_ActorPortrait_Sky" "None" :!class /Script/Engine.PrimitiveComponent))
  (Variables|Default|SetSky%20material _returnvalue)
  (CallFunction|RefreshSky "/Engine/EngineResources/GrayLightTextureCube.GrayLightTextureCube" "(R=1.000000,G=1.000000,B=1.000000,A=1.000000)" 0.0))